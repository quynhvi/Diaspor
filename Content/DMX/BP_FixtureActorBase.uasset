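; DMX fixture actor Blueprint with a DMX component and a point light, apparently an unfinished base for DMX-controlled lighting.
; Each Tick sets the light's intensity from an Intensity variable, which these graphs never write.
; BeginPlay queries fixture patch attribute values without using them, and the patch-received event is empty.
; Disconnected nodes hold an unfinished mapping from attribute values to light intensity.
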(event OnFixturePatchReceived(DMX)
  (params (FixturePatch :type DMX%20Entity%20Fixture%20Patch%20Object%20Reference) (ValuePerAttribute :type DMX%20Normalized%20Attribute%20Value%20Map%20Structure%20%28by%20ref%29)))

(event Collision|EventActorBeginOverlap
  (params (OtherActor :type Actor%20Object%20Reference)))

(event EventTick
  (params (DeltaSeconds :type Float%20%28single-precision%29))
  (Rendering|Components|Light|SetIntensity (Variables|Default|GetPointLight) (Variables|Default|GetIntensity)))

(event EventBeginPlay
  (Class|DMXEntityFixturePatch|GetNormalizedAttributesValues (Class|DMXComponent|GetFixturePatch (Variables|Default|GetDMX)))
  (bind _outattributesmap (|GetDMXAttributeValues)))

(fn ConstructionScript)